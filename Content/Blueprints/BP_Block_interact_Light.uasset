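; Interactable light block that toggles its glow by driving the LightAmount scalar parameter on its Material.
; Each Interact call advances a FlipFlop that selects between off and on values, with the first call switching it off.
; On BeginPlay, after the parent logic, it calls Interact once if StartEnabled is false, so the block begins unlit.
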(event `self.ReceiveBeginPlay`
  (`parent.ReceiveBeginPlay`)
  (if (not (`self.StartEnabled`))
    (`self.Interact`)))

(event `self.Interact`
  (bind _isa (`/Engine/EditorBlueprintResources/StandardMacros.FlipFlop`)
    (:`A`
      _)
    (:`B`
      _))
  (`MaterialInstanceDynamic.SetScalarParameterValue` (`self.Material`) "LightAmount" (`KismetMathLibrary.SelectFloat` 0.0 1.0 _isa)))

(fn `UserConstructionScript`
  (`parent.UserConstructionScript`))