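; BP_Block_Chest is a chest block that opens and closes when interacted with.
; On BeginPlay it runs the parent logic, then applies the Material variable to the SMChestTop lid mesh.
; Each Interact event alternates through a FlipFlop that sets IsOpen and plays or reverses the OpenClose timeline, which drives the pitch of the Scene component to animate the chest.
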(event `self.ReceiveBeginPlay`
  (`parent.ReceiveBeginPlay`)
  (`PrimitiveComponent.SetMaterial` (`self.SM_Chest_Top`) 0 (`self.Material`)))

(event `self.Interact`
  ;[1 1 1] Open / Close Chest
  (bind _isa (`/Engine/EditorBlueprintResources/StandardMacros.FlipFlop`)
    (:`A`
      (set `self.Is Open` _isa)
      (bind (_direction _rotation) (`Timeline|OpenClose` :!label _label)
        (:`Update`
          (`SceneComponent.K2_SetRelativeRotation` (`self.Scene`) (`KismetMathLibrary.MakeRotator` 0.0 _rotation) false false))))
    (:`B`
      (set `self.Is Open` _isa)
      (goto _label :!via `Reverse`))))

(fn `UserConstructionScript`
  (`parent.UserConstructionScript`))