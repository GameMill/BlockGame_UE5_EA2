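; BP_Block is a block actor that can be progressively destroyed, with the process reversible until it completes.
; On BeginPlay it creates a dynamic material on the Block component and sets the destroy timeline's play rate from DestoryPlayrate.
; StartDestroy plays the timeline to drive the DestoryAmount material parameter, destroying the actor on forward completion, while StopDestory reverses it.
; CanInteractLeft and CanInteractRight both return false.
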(event `self.ReceiveBeginPlay`
  ;[1 1 1] Begin Play - Create Dynamic Material Instance
  (bind _returnvalue (`PrimitiveComponent.CreateDynamicMaterialInstance` (`self.Block`) 0 null "None"))
  (set `self.Material` _returnvalue)
  (`TimelineComponent.SetPlayRate` (`self.DestoryTimeline`) (`self.DestoryPlayrate`)))

(event `StartDestroy`
  ;[1 1 1] Start / Stop Destroying Block
  (bind (_direction _destoyamount) (`Timeline|DestoryTimeline` :!label _label)
    (:`Update`
      (`MaterialInstanceDynamic.SetScalarParameterValue` (`self.Material`) "DestoryAmount" _destoyamount))
    (:`Finished`
      (if (`|EnumEquality` _direction "Forward")
        (`self.K2_DestroyActor`)))))

(event `StopDestory`
  ;[1 1 1] Start / Stop Destroying Block
  (goto _label :!via `Reverse`))

(fn `CanInteractLeft`
  (returns (CanInteract :type Boolean))
  (return false))

(fn `CanInteractRight`
  (returns (CanInteract :type Boolean))
  (return false))

(fn `UserConstructionScript`)